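; Team flag actor that third-person characters pick up or release on overlap, as in capture-the-flag.
; On overlap it accepts only the ThirdPersonCharacter class and compares its team with the flag's.
; An opposing character gets the flag attached and its CarriesFlag set.
; A same-team character detaches the flag in place and clears its own CarriesFlag, as the carry check there has empty branches.
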(event `self.ReceiveActorBeginOverlap`
  (params (OtherActor :type "Actor Object Reference"))
  (if (== (`GameplayStatics.GetObjectClass` OtherActor) "/Game/ThirdPerson/Blueprints/ThirdPersonCharacter.ThirdPersonCharacter_C")
    (bind _asthird_person_character (cast `/Game/ThirdPerson/Blueprints/ThirdPersonCharacter` OtherActor))
    (if (== (`self.team`) (`/Game/ThirdPerson/Blueprints/ThirdPersonCharacter.team` _asthird_person_character))
      (if (`/Game/ThirdPerson/Blueprints/ThirdPersonCharacter.carriesFlag` _asthird_person_character)
        _
        (else
          _))
      (`self.DetachRootComponentFromParent` true)
      (set `/Game/ThirdPerson/Blueprints/ThirdPersonCharacter.carriesFlag` false _asthird_person_character)
      (else
        (`self.K2_AttachRootComponentToActor` _asthird_person_character)
        (set `/Game/ThirdPerson/Blueprints/ThirdPersonCharacter.carriesFlag` true _asthird_person_character)))))

(fn `UserConstructionScript`)